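; BP_Planet is a configurable planet actor with surface, ring and atmosphere components, styled through exposed variables.
; Its Construction Script creates a dynamic material instance for each component and pushes in texture, terrain, ocean, ice, shadow, cloud and ring settings, plus layer visibility.
; All three materials take their light direction from a referenced DirectionalLight actor's rotation.
; A self-resetting RefreshMaterial bool re-runs construction from the Details panel; no runtime logic exists.
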(event EventBeginPlay)

(event Collision|EventActorBeginOverlap
  (params (OtherActor :type Actor%20Object%20Reference)))

(event EventTick
  (params (DeltaSeconds :type Float%20%28single-precision%29)))

(fn ConstructionScript
  (bind _directional_light_actor (Variables|SunSettings|GetDirectional%20light%20actor))
  (bind _atmosphere_visibility (Variables|CloudSettings|GetAtmosphere%20Visibility))
  (bind _rings_visibility (Variables|RingsSettings|GetRings%20Visibility))
  (bind _rings (Variables|Default|GetRings))
  (bind _texture_array (Variables|Default|GetTexture_Array))
  (bind _atmosphere (Variables|Default|GetAtmosphere))
  (bind _returnvalue (Transformation|GetActorRotation _directional_light_actor))
  (bind _returnvalue_2 (Math|Rotator|GetRotationXVector _returnvalue))
  (bind _returnvalue_3 (Math|Conversions|ToLinearColor(Vector) _returnvalue_2))
  (bind _returnvalue_4 (Rendering|Material|CreateDynamicMaterialInstance (Variables|Default|GetPlanet) 0 "/Game/Planet_Generator/Materials/M_SurfacePlanet.M_SurfacePlanet" "None" :!class /Script/Engine.PrimitiveComponent))
  (Variables|Default|SetPlanet%20Surface%20Material _returnvalue_4)
  (bind _returnvalue_5 (Rendering|Material|CreateDynamicMaterialInstance (Variables|Default|GetRings) 0 "/Game/Planet_Generator/Materials/M_RingPlanet.M_RingPlanet" "None" :!class /Script/Engine.PrimitiveComponent))
  (Variables|Default|SetRing%20Planet%20Material _returnvalue_5)
  (bind _returnvalue_6 (Rendering|Material|CreateDynamicMaterialInstance (Variables|Default|GetAtmosphere) 0 "/Game/Planet_Generator/Materials/M_Cloud.M_Cloud" "None" :!class /Script/Engine.PrimitiveComponent))
  (Variables|Default|SetAtmosphere%20Planet%20Material _returnvalue_6)
  (if (Variables|SunSettings|GetRefreshMaterial) ; Updating bool in details panel causes construction script to run again
    _
    (else
      _))
  (Variables|SunSettings|SetRefreshMaterial false)
  (Utilities|FlowControl|Sequence
    (:then_0
      ;[1 1 1] Sun Direction
      (Rendering|Material|SetVectorParameterValue (Variables|Default|GetPlanet%20Surface%20Material) "Light direction" _returnvalue_3 :!class /Script/Engine.MaterialInstanceDynamic)
      (Rendering|Material|SetVectorParameterValue (Variables|Default|GetRing%20Planet%20Material) "Light direction" _returnvalue_3 :!class /Script/Engine.MaterialInstanceDynamic)
      (Rendering|Material|SetVectorParameterValue (Variables|Default|GetAtmosphere%20Planet%20Material) "Light direction" _returnvalue_3 :!class /Script/Engine.MaterialInstanceDynamic))
    (:then_1
      ;[1 1 1] Cloud Settings
      (Rendering|SetVisibility _atmosphere _atmosphere_visibility false)
      (Development|SetHiddeninGame _atmosphere (not _atmosphere_visibility) false)
      (Rendering|Material|SetVectorParameterValue (Variables|Default|GetAtmosphere%20Planet%20Material) "Cloud Variant" (Utilities|Select :Index (Variables|CloudSettings|GetCloud%20Variant) :Option%200 "(R=1.000000,G=0.000000,B=0.000000,A=1.000000)" :Option%201 "(R=0.000000,G=1.000000,B=0.000000,A=1.000000)" :Option%202 "(R=0.000000,G=0.000000,B=1.000000,A=1.000000)") :!class /Script/Engine.MaterialInstanceDynamic)
      (Rendering|Material|SetVectorParameterValue (Variables|Default|GetAtmosphere%20Planet%20Material) "Color_Cloud" (Variables|CloudSettings|GetColor%20Cloud) :!class /Script/Engine.MaterialInstanceDynamic)
      (Rendering|Material|SetVectorParameterValue (Variables|Default|GetAtmosphere%20Planet%20Material) "Color_Atmosphere" (Variables|CloudSettings|GetColor%20Atmosphere) :!class /Script/Engine.MaterialInstanceDynamic)
      (Rendering|Material|SetScalarParameterValue (Variables|Default|GetAtmosphere%20Planet%20Material) "Cloud_Speed" (Math|Float|MapRangeClamped (Variables|CloudSettings|GetCloud_Speed) 0.0 1.0 0.0 0.001) :!class /Script/Engine.MaterialInstanceDynamic)
      (Rendering|Material|SetScalarParameterValue (Variables|Default|GetAtmosphere%20Planet%20Material) "Power_Cloud" (Variables|CloudSettings|GetPower_Cloud) :!class /Script/Engine.MaterialInstanceDynamic)
      (Rendering|Material|SetScalarParameterValue (Variables|Default|GetAtmosphere%20Planet%20Material) "Exponent_Cloud" (Variables|CloudSettings|GetExponent_Cloud) :!class /Script/Engine.MaterialInstanceDynamic)
      (Rendering|Material|SetScalarParameterValue (Variables|Default|GetAtmosphere%20Planet%20Material) "Edge_Brightness_Cloud" (Variables|CloudSettings|GetEdge_Brightness_Cloud) :!class /Script/Engine.MaterialInstanceDynamic)
      (Rendering|Material|SetScalarParameterValue (Variables|Default|GetAtmosphere%20Planet%20Material) "Exponent_Atmosphere" (Variables|CloudSettings|GetExponent_Atmosphere) :!class /Script/Engine.MaterialInstanceDynamic)
      (Rendering|Material|SetScalarParameterValue (Variables|Default|GetAtmosphere%20Planet%20Material) "Edge_Brightness_Atmosphere" (Variables|CloudSettings|GetEdge_Brightness_Atmosphere) :!class /Script/Engine.MaterialInstanceDynamic)
      (Rendering|Material|SetScalarParameterValue (Variables|Default|GetAtmosphere%20Planet%20Material) "Opasity_Atmosphere" (Variables|CloudSettings|GetOpasity_Atmosphere) :!class /Script/Engine.MaterialInstanceDynamic)
      (Rendering|Material|SetScalarParameterValue (Variables|Default|GetAtmosphere%20Planet%20Material) "Cloud_Brightness" (Variables|CloudSettings|GetCloud_Brightness) :!class /Script/Engine.MaterialInstanceDynamic))
    (:then_2
      ;[1 1 1] Rings Settings
      (Rendering|SetVisibility _rings _rings_visibility false)
      (Development|SetHiddeninGame _rings (not _rings_visibility) false)
      (Rendering|Material|SetVectorParameterValue (Variables|Default|GetRing%20Planet%20Material) "Color_01" (Variables|RingsSettings|GetColor_01) :!class /Script/Engine.MaterialInstanceDynamic)
      (Rendering|Material|SetVectorParameterValue (Variables|Default|GetRing%20Planet%20Material) "Color_02" (Variables|RingsSettings|GetColor_02) :!class /Script/Engine.MaterialInstanceDynamic)
      (Rendering|Material|SetVectorParameterValue (Variables|Default|GetRing%20Planet%20Material) "Color_03" (Variables|RingsSettings|GetColor_03) :!class /Script/Engine.MaterialInstanceDynamic)
      (Rendering|Material|SetScalarParameterValue (Variables|Default|GetRing%20Planet%20Material) "Frequency_Rings_Colors" (Variables|RingsSettings|GetFrequency_Rings_Colors) :!class /Script/Engine.MaterialInstanceDynamic)
      (Rendering|Material|SetVectorParameterValue (Variables|Default|GetRing%20Planet%20Material) "Color_Scattering" (Variables|RingsSettings|GetColor_Scattering) :!class /Script/Engine.MaterialInstanceDynamic)
      (Rendering|Material|SetScalarParameterValue (Variables|Default|GetRing%20Planet%20Material) "Ring_Scattering_Strength" (Variables|RingsSettings|GetRing_Scattering_Strength) :!class /Script/Engine.MaterialInstanceDynamic)
      (Rendering|Material|SetScalarParameterValue (Variables|Default|GetRing%20Planet%20Material) "Shadow_Rings_Blur" (Variables|RingsSettings|GetShadow_Rings_Blur) :!class /Script/Engine.MaterialInstanceDynamic)
      (Rendering|Material|SetScalarParameterValue (Variables|Default|GetRing%20Planet%20Material) "Shadow_Rings_Intensity" (Variables|RingsSettings|GetShadow_Rings_Intensity) :!class /Script/Engine.MaterialInstanceDynamic)
      (Rendering|Material|SetScalarParameterValue (Variables|Default|GetRing%20Planet%20Material) "Outer_Radius" (Variables|RingsSettings|GetOuter_Radius) :!class /Script/Engine.MaterialInstanceDynamic)
      (Rendering|Material|SetScalarParameterValue (Variables|Default|GetRing%20Planet%20Material) "Inner_Radius" (Variables|RingsSettings|GetInner_Radius) :!class /Script/Engine.MaterialInstanceDynamic)
      (Rendering|Material|SetScalarParameterValue (Variables|Default|GetRing%20Planet%20Material) "Edge_Blur" (Variables|RingsSettings|GetEdge_Blur) :!class /Script/Engine.MaterialInstanceDynamic)
      (Rendering|Material|SetScalarParameterValue (Variables|Default|GetRing%20Planet%20Material) "Frequency_Rings" (Variables|RingsSettings|GetFrequency_Rings) :!class /Script/Engine.MaterialInstanceDynamic)
      (Rendering|Material|SetScalarParameterValue (Variables|Default|GetRing%20Planet%20Material) "Position_Rings" (Variables|RingsSettings|GetPosition_Rings) :!class /Script/Engine.MaterialInstanceDynamic)
      (Rendering|Material|SetScalarParameterValue (Variables|Default|GetRing%20Planet%20Material) "Opacity_Rings" (Variables|RingsSettings|GetOpacity_Rings) :!class /Script/Engine.MaterialInstanceDynamic))
    (:then_3
      ;[1 1 1] Planet Texture Settings
      (Rendering|Material|SetTextureParameterValue (Variables|Default|GetPlanet%20Surface%20Material) "Texture_01" (Utilities|ResolveSoftReference (Utilities|Array|Get(acopy) _texture_array (- (Variables|PlanetSettings|GetFirst%20Texture%20Variant) 1))))
      (Rendering|Material|SetTextureParameterValue (Variables|Default|GetPlanet%20Surface%20Material) "Texture_02" (Utilities|ResolveSoftReference (Utilities|Array|Get(acopy) _texture_array (- (Variables|PlanetSettings|GetSecond%20Texture%20Variant) 1))))
      (Rendering|Material|SetScalarParameterValue (Variables|Default|GetPlanet%20Surface%20Material) "PlanetScale" (Variables|PlanetSettings|GetTexture%20Scale) :!class /Script/Engine.MaterialInstanceDynamic))
    (:then_4
      ;[1 1 1] Color Terrain
      (Rendering|Material|SetVectorParameterValue (Variables|Default|GetPlanet%20Surface%20Material) "Color_Terrain_01_Layer" (Variables|PlanetSettings|GetColor_Terrain_01) :!class /Script/Engine.MaterialInstanceDynamic)
      (Rendering|Material|SetVectorParameterValue (Variables|Default|GetPlanet%20Surface%20Material) "Color_Terrain_02_Layer" (Variables|PlanetSettings|GetColor_Terrain_02) :!class /Script/Engine.MaterialInstanceDynamic)
      ;[1 1 1] Ice
      (Rendering|Material|SetScalarParameterValue (Variables|Default|GetPlanet%20Surface%20Material) "Power_Equator_Zone" (Variables|PlanetSettings|GetIcing_Zone) :!class /Script/Engine.MaterialInstanceDynamic)
      (Rendering|Material|SetScalarParameterValue (Variables|Default|GetPlanet%20Surface%20Material) "Contrast_Equator_Zone" (Variables|PlanetSettings|GetIcing_Zone_Contrast) :!class /Script/Engine.MaterialInstanceDynamic)
      (Rendering|Material|SetVectorParameterValue (Variables|Default|GetPlanet%20Surface%20Material) "Color_Ice_Layer_01" (Variables|PlanetSettings|GetIce_Color_01) :!class /Script/Engine.MaterialInstanceDynamic)
      (Rendering|Material|SetVectorParameterValue (Variables|Default|GetPlanet%20Surface%20Material) "Color_Ice_Layer_02" (Variables|PlanetSettings|GetIce_Color_02) :!class /Script/Engine.MaterialInstanceDynamic)
      ;[1 1 1] Ocean
      (Rendering|Material|SetScalarParameterValue (Variables|Default|GetPlanet%20Surface%20Material) "Ocean_Level" (Variables|PlanetSettings|GetOcean_Level) :!class /Script/Engine.MaterialInstanceDynamic)
      (Rendering|Material|SetScalarParameterValue (Variables|Default|GetPlanet%20Surface%20Material) "Ocean_Noize" (Variables|PlanetSettings|GetOcean_Noize) :!class /Script/Engine.MaterialInstanceDynamic)
      (Rendering|Material|SetVectorParameterValue (Variables|Default|GetPlanet%20Surface%20Material) "Color_Ocean_Layer_01" (Variables|PlanetSettings|GetColor_Ocean) :!class /Script/Engine.MaterialInstanceDynamic)
      (Rendering|Material|SetVectorParameterValue (Variables|Default|GetPlanet%20Surface%20Material) "Color_Ocean_Layer_02" (Variables|PlanetSettings|GetColor_Ocean_Edge) :!class /Script/Engine.MaterialInstanceDynamic)
      (Rendering|Material|SetVectorParameterValue (Variables|Default|GetPlanet%20Surface%20Material) "Reflection_Color_Ocean" (Variables|PlanetSettings|GetReflection_Color_Ocean) :!class /Script/Engine.MaterialInstanceDynamic))
    (:then_5
      ;[1 1 1] Shadows
      (Rendering|Material|SetVectorParameterValue (Variables|Default|GetPlanet%20Surface%20Material) "Shadows_Color" (Variables|PlanetSettings|GetShadows_Color) :!class /Script/Engine.MaterialInstanceDynamic)
      (Rendering|Material|SetScalarParameterValue (Variables|Default|GetPlanet%20Surface%20Material) "Shadows_Intensity" (Variables|PlanetSettings|GetShadows_Intensity) :!class /Script/Engine.MaterialInstanceDynamic)
      ;[1 1 1] Atmosphere
      (Rendering|Material|SetVectorParameterValue (Variables|Default|GetPlanet%20Surface%20Material) "Color_Atmosphere" (Variables|PlanetSettings|GetColor_Atmosphere) :!class /Script/Engine.MaterialInstanceDynamic)
      (Rendering|Material|SetScalarParameterValue (Variables|Default|GetPlanet%20Surface%20Material) "Exponent_Atmosphere" (Variables|PlanetSettings|GetExponent_Atmosphere_Planet) :!class /Script/Engine.MaterialInstanceDynamic)
      (Rendering|Material|SetScalarParameterValue (Variables|Default|GetPlanet%20Surface%20Material) "Edge_Brightness_Atmosphere" (Variables|PlanetSettings|GetEdge_Brightness_Atmosphere_Planet) :!class /Script/Engine.MaterialInstanceDynamic)
      (Rendering|Material|SetScalarParameterValue (Variables|Default|GetPlanet%20Surface%20Material) "Brightness_Atmosphere" (Variables|PlanetSettings|GetBrightness_Atmosphere_Planet) :!class /Script/Engine.MaterialInstanceDynamic))))