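; Starfield backdrop actor for the planet generator that renders stars and a sun through a material on its Starfield component.
; The construction script creates a dynamic M_Starfield instance, derives the light direction from the referenced directional light's rotation, and applies sun and near/far star settings.
; RefreshMaterial acts as an editor button: toggling it reruns construction, which resets it to false.
; No runtime logic exists.
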(event EventBeginPlay)

(event Collision|EventActorBeginOverlap
  (params (OtherActor :type Actor%20Object%20Reference)))

(event EventTick
  (params (DeltaSeconds :type Float%20%28single-precision%29)))

(fn ConstructionScript
  (bind _returnvalue (Rendering|Material|CreateDynamicMaterialInstance (Variables|Default|GetStarfield) 0 "/Game/Planet_Generator/Materials/M_Starfield.M_Starfield" "None" :!class /Script/Engine.PrimitiveComponent))
  (Variables|Default|SetStarfieldMaterial _returnvalue)
  (if (Variables|SettingsSun|GetRefreshMaterial) ; Updating bool in details panel causes construction script to run again
    _
    (else
      _))
  (Variables|SettingsSun|SetRefreshMaterial false)
  ;[1 1 1] Sun settings
  (Rendering|Material|SetVectorParameterValue (Variables|Default|GetStarfieldMaterial) "Light direction" (Math|Conversions|ToLinearColor(Vector) (Math|Rotator|GetRotationXVector (Transformation|GetActorRotation (Variables|SettingsSun|GetDirectional%20light%20actor)))) :!class /Script/Engine.MaterialInstanceDynamic)
  (Rendering|Material|SetVectorParameterValue (Variables|Default|GetStarfieldMaterial) "Sun_Color" (Variables|SettingsSun|GetSun%20Color) :!class /Script/Engine.MaterialInstanceDynamic)
  (Rendering|Material|SetScalarParameterValue (Variables|Default|GetStarfieldMaterial) "Sun_Brightness" (Variables|SettingsSun|GetSun%20Brightness) :!class /Script/Engine.MaterialInstanceDynamic)
  (Rendering|Material|SetScalarParameterValue (Variables|Default|GetStarfieldMaterial) "Sun_Radius" (Variables|SettingsSun|GetSun%20Radius) :!class /Script/Engine.MaterialInstanceDynamic)
  ;[1 1 1] Star settings
  (Rendering|Material|SetScalarParameterValue (Variables|Default|GetStarfieldMaterial) "PowerStarsNear" (Variables|SettingsStars|GetPower%20Stars%20Near) :!class /Script/Engine.MaterialInstanceDynamic)
  (Rendering|Material|SetScalarParameterValue (Variables|Default|GetStarfieldMaterial) "IntensityStarsNear" (Variables|SettingsStars|GetIntensity%20Stars%20Near) :!class /Script/Engine.MaterialInstanceDynamic)
  (Rendering|Material|SetScalarParameterValue (Variables|Default|GetStarfieldMaterial) "PowerStarsFor" (Variables|SettingsStars|GetPower%20Stars%20For) :!class /Script/Engine.MaterialInstanceDynamic)
  (Rendering|Material|SetScalarParameterValue (Variables|Default|GetStarfieldMaterial) "IntensityStarsFor" (Variables|SettingsStars|GetIntensity%20Stars%20For) :!class /Script/Engine.MaterialInstanceDynamic))